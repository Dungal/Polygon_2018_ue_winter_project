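; BP_Obstacle is an obstacle actor that moves back and forth between EndPosition and the start location captured on BeginPlay.
; Each tick raises or lowers a 0–1 alpha by delta time over TimeOfTravel, flipping direction at the limits.
; NewFunction0 lerps from EndPosition to StartPosition without sweep, so movement begins at the end point rather than the placed location.
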(event EventTick
  (params (DeltaSeconds :type Float%20%28single-precision%29))
  (bind _timeoftravel (Variables|Default|GettimeOfTravel))
  (bind _returnvalue (/ DeltaSeconds _timeoftravel))
  ;[1 1 1] Moving back and forth
  (if (Variables|Default|GetisForward)
    (bind _output_get (Variables|Default|Settmp (+ _returnvalue (Variables|Default|Gettmp))))
    (Variables|Default|SetisForward (> 1.0 _output_get))
    (else
      (bind _output_get_2 (Variables|Default|Settmp (- (Variables|Default|Gettmp) _returnvalue)))
      (Variables|Default|SetisForward (> 0.0 _output_get_2))))
  (CallFunction|NewFunction0 (Variables|Default|Gettmp)))

(event EventBeginPlay
  ;[1 1 1] SetUP
  (Variables|Default|SetstartPosition (Transformation|GetActorLocation))
  (Variables|Default|Settmp 0.0)
  (Variables|Default|SetisForward true))

(fn ConstructionScript)

(fn NewFunction0
  (params (Alpha :type Float%20%28single-precision%29))
  (Transformation|SetActorLocation (Math|Vector|Lerp(Vector) (Variables|Default|GetendPosition) (Variables|Default|GetstartPosition) Alpha) false false))